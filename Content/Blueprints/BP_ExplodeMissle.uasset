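; Missile projectile that orients to its fire direction, plays flight audio and a Niagara smoke trail, and explodes on static world geometry.
; Tick moves it by a fixed per-frame offset without sweep or delta-time scaling.
; WorldStatic hits spawn an explosion facing the stored helicopter location, a fading randomly rotated decal and sound, removing mesh, then trail.
; The actor destroys itself when the explosion particles finish or its lifetime expires.
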(event OnComponentHit(SM_Missle)
  (params (HitComponent :type Primitive%20Component%20Object%20Reference) (OtherActor :type Actor%20Object%20Reference) (OtherComp :type Primitive%20Component%20Object%20Reference) (NormalImpulse :type Vector :default "0, 0, 0") (Hit :type Hit%20Result%20Structure%20%28by%20ref%29))
  (bind _location (Collision|BreakHitResult Hit))
  ;[0.7374 0.2108 1] 导弹撞击物体反应
  (if (Utilities|Enum|Equal(Enum) (Collision|GetCollisionObjectType OtherComp) "ECC_WorldStatic")
    (Utilities|FlowControl|Sequence
      (:then_0
        ;;[0.2399 0.03732 1] 播放爆破粒子
        (bind _returnvalue (Effects|SpawnEmitteratLocation (Variables|Components|GetP_Explosion) _location (Math|Rotator|FindLookatRotation _location (Variables|Default|GetHelicopterLocation))))
        (EventDispatchers|BindEventtoOnSystemFinished _returnvalue (delegate Custom|ExplodeFinish))
        (Components|DestroyComponent (Variables|Components|GetSM_Missle))
        (Utilities|FlowControl|Delay 2.0)
        (Components|DestroyComponent (Variables|Components|GetN_MissleSmoke)))
      (:then_1
        ;;[0 0.2196 1] 爆炸贴花
        (bind _returnvalue_2 (Rendering|Decal|SpawnDecalatLocation (Variables|Components|GetDecal_Ground) (Variables|Decal|GetDecalSize) _location (Math|Rotator|MakeRotator 0.0 9e+01 (Math|Random|RandomFloatinRange 0.0 3.6e+02)) 0.0))
        (Rendering|Components|Decal|SetFadeOut _returnvalue_2 4.0 6.0 true)
        ;;[0.296 0.135 1] 爆炸音效
        (Audio|Components|Audio|Play (Variables|Default|GetExplosion) 0.0)))))

(event Custom|ExplodeFinish
  (params (PSystem :type Particle%20System%20Component%20Object%20Reference))
  ;[0.7374 0.2108 1] 导弹撞击物体反应
  (EventDispatchers|UnbindallEventsfromOnSystemFinished (stale OnComponentHit(SM_Missle) _returnvalue))
  (Actor|DestroyActor))

(event EventBeginPlay
  (bind _sm_missle (Variables|Components|GetSM_Missle))
  (bind _returnvalue (Transformation|GetWorldLocation _sm_missle))
  (Utilities|FlowControl|Sequence
    (:then_0
      ;[0.6745 0.3728 1] 导弹朝向发射点
      (Transformation|SetWorldRotation (Variables|Components|GetSM_Missle) (Math|Rotator|FindLookatRotation _returnvalue (+ _returnvalue (Variables|Missle|GetFireDirection))) false false)
      ;[1 0.8109 0.01262] 设置尾焰速度
      (Class|NiagaraComponent|SetNiagaraVariableVec3 (Variables|Components|GetN_MissleSmoke) "User.FireDirection" (* (* (Variables|Missle|GetFireDirection) -1.0) (Variables|Missle|GetSmokeSpeed)))
      ;[1 0 0.7385] 播放飞行音效
      (Audio|Components|Audio|Play (Variables|Default|GetMissleFly) 0.0))
    (:then_1
      ;[1 0.1304 0] BUG
      (Transformation|AttachComponentToComponent (Variables|Components|GetSM_Missle) (Variables|Components|GetScene) "None" "KeepWorld" "KeepWorld" "KeepWorld" true))
    (:then_2
      ;[1 0.3991 0.9388] 长时间未命中目标销毁自己
      (Utilities|FlowControl|Delay (Variables|Missle|GetMissleLifetime))
      (Actor|DestroyActor))))

(event EventTick
  (params (DeltaSeconds :type Float%20%28single-precision%29))
  ;[0.8719 1 0.1168] 导弹飞行
  (Transformation|AddActorWorldOffset (* (Variables|Missle|GetFireDirection) (Variables|Missle|GetFireSpeed))))

(fn ConstructionScript)