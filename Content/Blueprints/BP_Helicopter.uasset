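; Player-controlled helicopter that flies with eased, inertial movement and fires missiles.
; Axis inputs feed interpolated velocities; Tick applies them as unswept offsets, tilts the body, turns the actor and spins the rotors.
; A ground overlap limits movement to lift-off and mutes the flight loop.
; The spring arm trails yaw and pitches with forward/back input; Fire launches two missiles toward a screen-centre trace, with camera shake.
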(event OnComponentBeginOverlap(IsOnGround)
  (params (OverlappedComponent :type Primitive%20Component%20Object%20Reference) (OtherActor :type Actor%20Object%20Reference) (OtherComp :type Primitive%20Component%20Object%20Reference) (OtherBodyIndex :type Integer) (bFromSweep :type Boolean) (SweepResult :type Hit%20Result%20Structure%20%28by%20ref%29))
  (if (Utilities|Enum|Equal(Enum) (Collision|GetCollisionObjectType OtherComp) "ECC_WorldStatic")
    (Variables|Default|SetbIsOnGround true)))

(event OnComponentEndOverlap(IsOnGround)
  (params (OverlappedComponent :type Primitive%20Component%20Object%20Reference) (OtherActor :type Actor%20Object%20Reference) (OtherComp :type Primitive%20Component%20Object%20Reference) (OtherBodyIndex :type Integer))
  (if (Utilities|Enum|Equal(Enum) (Collision|GetCollisionObjectType OtherComp) "ECC_WorldStatic")
    (Variables|Default|SetbIsOnGround false)))

(event EventTick
  (params (DeltaSeconds :type Float%20%28single-precision%29))
  (bind _returnvalue (Input|AxisValues|GetMoveForward))
  (bind _bisonground (Variables|Default|GetbIsOnGround))
  (bind _upnowv (Variables|Movement|GetUpNowV))
  (bind _returnvalue_2 (Math|Float|Clamp(Float) _upnowv -6e+01 6e+01))
  (bind _returnvalue_3 (Math|Float|SelectFloat _returnvalue_2 6e+01 _bisonground))
  (Variables|Default|SetDeltaTime DeltaSeconds)
  (CallFunction|CameraControl) ; 相机跟随与视角控制
  ;[0 1 0.1073] 直升机旋转
  (Transformation|SetRelativeRotation (Variables|Default|GetBody) (Math|Rotator|MakeRotator (Math|Interpolation|FInterpTo (.roll (Transformation|GetWorldRotation (Variables|Default|GetBody))) (Math|Float|SelectFloat (/ (Variables|Movement|GetRightNowV) (Variables|Rotate|GetBodyRotateClamp)) 0.0 (!= (Input|AxisValues|GetMoveForward) 0.0)) (Variables|Default|GetDeltaTime) (Variables|Rotate|GetRotateInterpSpeed)) (/ (* (Variables|Movement|GetForwardNowV) -1.0) (Variables|Rotate|GetBodyRotateClamp)) 0.0) false false)
  (Transformation|SetActorRotation (Math|Rotator|MakeRotator 0.0 0.0 (+ (.yaw (Transformation|GetActorRotation)) (* (/ (Math|Float|SelectFloat 0.0 (Input|AxisValues|GetMoveRight) (Variables|Default|GetbIsOnGround)) (Variables|Rotate|GetRootRotateClamp)) (Math|Float|SelectFloat _returnvalue 1.0 (!= _returnvalue 0.0))))))
  ;[1 0.05451 0] 直升机移动
  (Transformation|AddActorWorldOffset (+ (* (Transformation|GetActorForwardVector) (Variables|Movement|GetForwardNowV)) (Math|Vector|SelectVector (* (Transformation|GetActorRightVector) (Variables|Movement|GetRightNowV)) "0, 0, 0" (!= (Input|AxisValues|GetMoveForward) 0.0)) (* (Transformation|GetActorUpVector) (Variables|Movement|GetUpNowV))))
  ;[0.8145 0.3481 1] 螺旋桨逻辑
  (Transformation|AddRelativeRotation (Variables|Default|GetHead) (Math|Rotator|MakeRotator 0.0 0.0 _returnvalue_3) false false)
  (Transformation|AddRelativeRotation (Variables|Default|Gettail) (Math|Rotator|MakeRotator 0.0 _returnvalue_3 0.0) false false)
  ;[0 1 0.8478] 旋转音效
  (Components|Activation|SetActive (Variables|Default|GetFlyLoop) (not (Variables|Default|GetbIsOnGround)) false))

(event Input|ActionEvents|InputActionFire
  (params (Key :type Key%20Structure :default "None"))
  ;[1 0.4221 0] 发射导弹
  (:Pressed
    (CallFunction|FireMissle (Transformation|GetWorldLocation (Variables|Default|GetFireLocation)))
    (CallFunction|FireMissle (Transformation|GetWorldLocation (Variables|Default|GetFireLocation2)))
    ;;[1 0.6136 0.08228] 镜头晃动
    (Camera|PlayWorldCameraShake "/Game/Blueprints/BP_ExplosionShake.BP_ExplosionShake_C" (Transformation|GetActorLocation) 0.0 3e+03)))

(event Input|AxisEvents|InputAxisMoveForward
  (params (AxisValue :type Float%20%28single-precision%29))
  ;[1 0.3295 0.8479] 前后移动
  (Variables|Movement|SetForwardTargetV (* (Math|Float|SelectFloat 0.0 AxisValue (Variables|Default|GetbIsOnGround)) (Variables|Movement|GetMoveSpeed)))
  (Variables|Movement|SetForwardNowV (Math|Interpolation|FInterpTo (Variables|Movement|GetForwardNowV) (Variables|Movement|GetForwardTargetV) (Variables|Default|GetDeltaTime) (Variables|Movement|GetMoveInterpSpeed))))

(event Input|AxisEvents|InputAxisMoveRight
  (params (AxisValue :type Float%20%28single-precision%29))
  ;[0 1 0.7687] 左右移动
  (Variables|Movement|SetRightTargetV (* (Math|Float|SelectFloat 0.0 AxisValue (Variables|Default|GetbIsOnGround)) (/ (Variables|Movement|GetMoveSpeed) 2.0)))
  (Variables|Movement|SetRightNowV (Math|Interpolation|FInterpTo (Variables|Movement|GetRightNowV) (Variables|Movement|GetRightTargetV) (Variables|Default|GetDeltaTime) (Variables|Movement|GetMoveInterpSpeed))))

(event Input|AxisEvents|InputAxisMoveUp
  (params (AxisValue :type Float%20%28single-precision%29))
  ;[1 0.9884 0.1293] 上下移动
  (Variables|Movement|SetUpTargetV (* (Math|Float|SelectFloat (Math|Float|SelectFloat AxisValue 0.0 (> AxisValue 0.0)) AxisValue (Variables|Default|GetbIsOnGround)) (Variables|Movement|GetMoveSpeed)))
  (Variables|Movement|SetUpNowV (Math|Interpolation|FInterpTo (Variables|Movement|GetUpNowV) (Variables|Movement|GetUpTargetV) (Variables|Default|GetDeltaTime) (Variables|Movement|GetMoveInterpSpeed))))

(event Input|KeyboardEvents|LeftAlt
  (params (Key :type Key%20Structure :default "None"))
  ;[1 0 0.176] 相机自由视角开关
  (:Pressed
    (Variables|默认|SetbFreePerspective true))
  (:Released
    (Variables|默认|SetbFreePerspective false)))

(fn ConstructionScript)

(fn CameraControl
  (bind _returnvalue (Input|AxisValues|GetMoveForward))
  (Transformation|SetWorldRotation (Variables|Default|GetSpringArm) (Math|Rotator|MakeRotator 0.0 (Math|Interpolation|FInterpTo (.pitch (Transformation|GetWorldRotation (Variables|Default|GetSpringArm))) (Math|Float|SelectFloat (LocalVariables|GetDefaultPitch) (Math|Float|SelectFloat -6e+01 5.0 (> _returnvalue 0.0)) (or (== _returnvalue 0.0) (Variables|Default|GetbIsOnGround))) (Variables|Default|GetDeltaTime) (LocalVariables|GetFireInterpSpeed)) (Math|Interpolation|FInterpTo (.yaw (Transformation|GetWorldRotation (Variables|Default|GetSpringArm))) (.yaw (Transformation|GetActorRotation)) (Variables|Default|GetDeltaTime) (Variables|Rotate|GetRotateInterpSpeed))) false false) ; 相机视角
)

(fn FireMissle
  (params (Spawn%20Transform%20Location :type Vector))
  (bind _returnvalue (Viewport|GetViewportSize))
  (bind _returnvalue_2 (Viewport|GetViewportSize))
  (bind _returnvalue_3 (Game|GetPlayerCameraManager 0))
  (bind _returnvalue_4 (* _returnvalue 0.5))
  (bind _returnvalue_5 (* _returnvalue_2 0.5))
  (bind _returnvalue_6 (Camera|GetCameraLocation _returnvalue_3))
  ;[1 0.5304 0.2211] 射线检测获取导弹发射目标点
  (bind (_outhit _returnvalue_7) (Collision|LineTraceByChannel _returnvalue_6 (+ _returnvalue_6 (* (.WorldDirection (Class|GameplayStatics|DeprojectScreentoWorld (Game|GetPlayerController 0) (Math|Vector2D|MakeVector2D (.x _returnvalue_5) (.y _returnvalue_5)))) 1e+06)) "TraceTypeQuery1" false 0 "None"))
  (Game|SpawnActorfromClass "/Game/Blueprints/BP_ExplodeMissle.BP_ExplodeMissle_C" (Math|Transform|MakeTransform Spawn%20Transform%20Location "0, 0, 0" "1,1,1") "AlwaysSpawn" 0 (Transformation|GetActorLocation) (Math|Vector|SelectVector (Math|Vector|Normalize (- (.Location (Collision|BreakHitResult _outhit)) Spawn%20Transform%20Location)) (.WorldDirection (Class|GameplayStatics|DeprojectScreentoWorld (Game|GetPlayerController 0) (Math|Vector2D|MakeVector2D (.x _returnvalue_4) (.y _returnvalue_4)))) _returnvalue_7) 0))